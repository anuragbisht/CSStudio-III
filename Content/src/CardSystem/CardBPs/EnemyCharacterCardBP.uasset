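; Enemy character card actor that the player clicks to select as an attack target.
; On click, it blocks the attack with a debug message while any EnemyChildCardBP actor exists in the level.
; Otherwise it casts the controlled pawn to MyCharacter and calls ROSSetupCardTobeAttacked with index -1, registering the character card as the target.
; The construction script only calls its parent.
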(event EventBeginPlay)

(event Collision|EventActorBeginOverlap
  (params (OtherActor :type Actor%20Object%20Reference)))

(event EventTick
  (params (DeltaSeconds :type Float%20%28single-precision%29)))

(event MouseInput|EventActorOnClicked
  (params (ButtonPressed :type Key%20Structure :default "None"))
  ;[1 1 1] check if enemy character card can be attacked or not, if length > 0 it cannot
  (bind _outactors (Actor|GetAllActorsOfClass "/Game/src/CardSystem/CardBPs/EnemyChildCardBP.EnemyChildCardBP_C"))
  (if (> (Utilities|Array|Length _outactors) 0)
    (Development|PrintString "Cannot Attack ")
    (else
      ;[1 1 1] set character card in the attack handler
      (bind _asmy_character (Utilities|Casting|CastToMyCharacter (Pawn|GetControlledPawn (Game|GetPlayerController 0))))
      (Default|ROSSetupCardTobeAttacked _asmy_character -1))))

(fn ConstructionScript
  (|CallParentFunction))