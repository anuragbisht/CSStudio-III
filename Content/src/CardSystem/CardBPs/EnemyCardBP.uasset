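; EnemyCardBP is a clickable enemy card actor that shows its card data and triggers an attack from the player's pawn.
; The construction script fills the name, HP, AP and description text blocks from the Card struct.
; Clicking prints the card's Id and calls ROSAttack on the controlled MyCharacter.
; Hover events and ChangeTheLookOfCard are empty, and logic for applying AP, freeing a hand slot and destroying the card is disconnected.
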(event MouseInput|EventActorBeginCursorOver)

(event MouseInput|EventActorEndCursorOver)

(event MouseInput|EventActorOnClicked
  (params (ButtonPressed :type Key%20Structure :default "None"))
  (Development|PrintString (Utilities|String|ToString(Integer) (Variables|Default|GetId)))
  (bind _asmy_character (Utilities|Casting|CastToMyCharacter (Pawn|GetControlledPawn (Game|GetPlayerController 0))))
  (Default|ROSAttack _asmy_character))

(fn ConstructionScript
  (bind _card (Variables|Default|Getcard))
  (bind (_type _name _hitpoints _manapoints _attackpoints _shield _armor _description) (Utilities|Struct|BreakCard _card))
  (Rendering|Components|TextRender|SetText (Variables|Default|GetNameTextBlock) (Utilities|Text|ToText(String) _name))
  (Rendering|Components|TextRender|SetText (Variables|Default|GetHPTextBlock) (Utilities|Text|ToText(Integer) _hitpoints))
  (Rendering|Components|TextRender|SetText (Variables|Default|GetDescriptionTextBlock) (Utilities|Text|ToText(String) _description))
  (Rendering|Components|TextRender|SetText (Variables|Default|GetAPTextBlock) (Utilities|Text|ToText(Integer) _attackpoints)))

(fn ChangetheLookOfCard)