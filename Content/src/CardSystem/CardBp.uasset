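; Card actor for the card system that displays a card's sprite, name, description and HP, mana and attack values.
; The construction script fills the Paper sprite and text blocks from the Card struct.
; The cube click event and ChangeTheLookOfCard are empty.
; Unconnected graph logic would apply attack points to matching player characters, free the spawn point at the card's location and destroy the card.
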(event OnClicked(Cube)
  (params (TouchedComponent :type Primitive%20Component%20Object%20Reference) (ButtonPressed :type Key%20Structure :default "None")))

(fn ConstructionScript
  (bind _card (Variables|Default|Getcard))
  (bind (_type _name _hitpoints _manapoints _attackpoints _shield _armor _description _sprite) (Utilities|Struct|BreakCard _card))
  (Rendering|Components|Sprite|SetSprite (Variables|Default|GetPaperSprite) _sprite)
  (Rendering|Components|TextRender|SetText (Variables|Default|GetNameTextBlock) (Utilities|Text|ToText(String) _name))
  (Rendering|Components|TextRender|SetText (Variables|Default|GetHPTextBlock) (Utilities|Text|ToText(Integer) _hitpoints))
  (Rendering|Components|TextRender|SetText (Variables|Default|GetManaTextBlock) (Utilities|Text|ToText(Integer) _manapoints))
  (Rendering|Components|TextRender|SetText (Variables|Default|GetDescriptionTextBlock) (Utilities|Text|ToText(String) _description))
  (Rendering|Components|TextRender|SetText (Variables|Default|GetAPTextBlock) (Utilities|Text|ToText(Integer) _attackpoints)))

(fn ChangetheLookOfCard)