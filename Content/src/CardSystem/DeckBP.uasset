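; Clickable deck actor for the card system that draws cards from the player character's deck and shows a card count.
; Construction copies the Deck from the matching YinPlayerCharacter1 and displays its size minus five.
; Clicking the cube checks for an available spawn target point and fewer than five CardBP actors.
; If allowed, the character spawns cards at each available point and the count text refreshes; otherwise it prints a refusal.
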(event OnClicked(Cube)
  (params (TouchedComponent :type Primitive%20Component%20Object%20Reference) (ButtonPressed :type Key%20Structure :default "None"))
  (CallFunction|DrawCard))

(event EventBeginPlay)

(event Collision|EventActorBeginOverlap
  (params (OtherActor :type Actor%20Object%20Reference)))

(event EventTick
  (params (DeltaSeconds :type Float%20%28single-precision%29)))

(fn ConstructionScript
  (CallFunction|SetupDeck))

(fn SetupDeck
  (bind _outactors (Actor|GetAllActorsOfClass "/Game/src/Characters/PlayerCharacter/YinPlayerCharacter1.YinPlayerCharacter1_C"))
  (for _array_element _outactors
    (if (Utilities|Enum|Equal(Enum) (Variables|/Game/src/Characters/PlayerCharacter/YinPlayerCharacter1.YinPlayerCharacter1_C|GetCharacterType _array_element) "NewEnumerator0")
      (bind _output_get (Variables|Default|SetDeck (Variables|/Game/src/Characters/PlayerCharacter/YinPlayerCharacter1.YinPlayerCharacter1_C|GetDeck _array_element)))
      (Rendering|Components|TextRender|SetText (Variables|Default|GetNumberOfCArdsTextRenderer) (Utilities|Text|ToText(Integer) (- (Utilities|Array|Length _output_get) 5))))))

(fn DrawCard
  (params (TargetPoint :type Target%20Point%20Object%20Reference))
  (CallFunction|IsDrawAllowed)
  (if (Variables|Default|GetCanCardBeDrawn)
    (Utilities|FlowControl|Sequence
      (:then_0
        (bind _outactors (Actor|GetAllActorsOfClass "/Game/src/CardSystem/CardSpawnLocationTargetPoint.CardSpawnLocationTargetPoint_C"))
        (for _array_element _outactors
          (if (Variables|/Game/src/CardSystem/CardSpawnLocationTargetPoint.CardSpawnLocationTargetPoint_C|GetIsAvailable _array_element)
            (Variables|Default|SetTargetPointToDrawCard _array_element)
            (bind _outactors_2 (Actor|GetAllActorsOfClass "/Game/src/Characters/PlayerCharacter/YinPlayerCharacter1.YinPlayerCharacter1_C"))
            (for _array_element_2 _outactors_2
              (if (Utilities|Enum|Equal(Enum) (Variables|/Game/src/Characters/PlayerCharacter/YinPlayerCharacter1.YinPlayerCharacter1_C|GetCharacterType _array_element_2) "NewEnumerator0")
                (Default|SpawnCardsatTargetPosition _array_element_2 (Variables|Default|GetTargetPointToDrawCard))
                (CallFunction|UpdateDeckCardNumberText)))))))
    (else
      (Development|PrintString "DrawNotAllowed"))))

(fn IsDrawAllowed
  (bind _outactors (Actor|GetAllActorsOfClass "/Game/src/CardSystem/CardSpawnLocationTargetPoint.CardSpawnLocationTargetPoint_C"))
  (for _array_element _outactors
    (if (Variables|/Game/src/CardSystem/CardSpawnLocationTargetPoint.CardSpawnLocationTargetPoint_C|GetIsAvailable _array_element)
      (bind _outactors_2 (Actor|GetAllActorsOfClass "/Game/src/CardSystem/CardBp.CardBP_C"))
      (if (< (Utilities|Array|Length _outactors_2) 5)
        (Variables|Default|SetCanCardBeDrawn true)
        (return)
        (else
          (Variables|Default|SetCanCardBeDrawn false)))
      (else
        (Variables|Default|SetCanCardBeDrawn false)))))

(fn GetTargetPointtoDrawCard)

(fn UpdateDeckCardNumberText
  (bind _outactors (Actor|GetAllActorsOfClass "/Game/src/Characters/PlayerCharacter/YinPlayerCharacter1.YinPlayerCharacter1_C"))
  (for _array_element _outactors
    (if (Utilities|Enum|Equal(Enum) (Variables|/Game/src/Characters/PlayerCharacter/YinPlayerCharacter1.YinPlayerCharacter1_C|GetCharacterType _array_element) "NewEnumerator0")
      (Rendering|Components|TextRender|SetText (Variables|Default|GetNumberOfCArdsTextRenderer) (Utilities|Text|ToText(Integer) (Utilities|Array|Length (Variables|/Game/src/Characters/PlayerCharacter/YinPlayerCharacter1.YinPlayerCharacter1_C|GetDeck _array_element)))))))