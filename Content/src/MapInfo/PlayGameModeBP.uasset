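; PlayGameModeBP is a game mode Blueprint that tracks whose turn it is in a turn-based match.
; ChangeTurn toggles the Turn enum, switching to the second value from the first and otherwise resetting to the first.
; Turn uses RepNotify, so OnRep_Turn prints the new turn as debug text and broadcasts it through the ChangeOfTurn dispatcher.
; BeginPlay and the construction script are empty.
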(event Custom|ChangeTurn
  ;[1 1 1] changes the turn variable
  (if (Utilities|Enum|Equal(Enum) (Variables|Playerinfo|GetTurn) "NewEnumerator0")
    (Variables|Playerinfo|SetTurn "NewEnumerator1")
    (else
      (Variables|Playerinfo|SetTurn "NewEnumerator0"))))

(event EventBeginPlay)

(fn ConstructionScript)

(fn OnRepTurn
  (bind _turn (Variables|Playerinfo|GetTurn))
  (Development|PrintString (Utilities|String|Append "the turn is of " (Utilities|String|EnumtoString _turn)))
  (Default|CallChangeOfTurn _turn))