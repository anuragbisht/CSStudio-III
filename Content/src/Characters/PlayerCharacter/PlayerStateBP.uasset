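; Player state Blueprint that relays a player's attack press through events named for server and multicast replication.
; AttackRunonserver calls AttackMulticast, which prints a debug message and calls AttackButtonPressed.
; AttackButtonPressed is empty as wired, so the relay has no gameplay effect.
; Its unconnected logic would cast the pawn to MyCharacter, call ChangeAttackButton with false and print the player's name.
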(event Custom|AttackRunonserver
  (CallFunction|AttackMulticast))

(event Custom|AttackMulticast
  (Development|PrintString "Attack  multicast called")
  (CallFunction|AttackButtonPressed))

(event EventBeginPlay)

(fn ConstructionScript)

(fn AttackButtonPressed)