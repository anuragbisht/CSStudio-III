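; Game state Blueprint with a Show Player List function that counts players and disables their attack buttons.
; The function loops over PlayerArray, counting every entry and casting its pawn to MyCharacter to disable that character's AttackButton, then prints the total.
; BeginPlay and the construction script do nothing, and leftover debug prints are disconnected.
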(event EventBeginPlay)

(fn ConstructionScript)

(fn ShowPlayerList
  (Variables|Default|Setcount%20 0)
  (for _array_element (Variables|Default|GetPlayerArray)
    (Math|Integer|IncrementInt (Variables|Default|Getcount%20)
      (:%20%20
        (bind _asmy_character (Utilities|Casting|CastToMyCharacter (Variables|/Script/Engine.PlayerState|GetPawnPrivate _array_element)))
        (Widget|SetIsEnabled (Variables|/Game/src/Characters/PlayerCharacter/MyCharacter.MyCharacter_C|GetAttackButton _asmy_character) false))))
  (Development|PrintString (Utilities|String|Append "number of players" (Utilities|String|ToString(Integer) (Variables|Default|Getcount%20)))))