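; Player controller Blueprint that identifies the opposing player's character when play begins.
; On BeginPlay it loops over the GameState PlayerArray and casts each pawn that is not locally controlled to MyCharacter.
; Each match overwrites the Opponent reference, as the loop has no break, and prints the opponent's name for debugging.
; The lookup runs only once, with no retry for pawns that arrive later.
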(event EventBeginPlay
  (for _array_element (Variables|/Script/Engine.GameStateBase|GetPlayerArray (Game|GetGameState))
    (if (not (Pawn|IsLocallyControlled (Variables|/Script/Engine.PlayerState|GetPawnPrivate _array_element)))
      (bind _asmy_character (Utilities|Casting|CastToMyCharacter (Variables|/Script/Engine.PlayerState|GetPawnPrivate _array_element)))
      (bind _output_get (Variables|Default|Setopponent _asmy_character))
      (Development|PrintString (Utilities|String|Append "opponent is " (Utilities|GetDisplayName _output_get))))))

(fn ConstructionScript)