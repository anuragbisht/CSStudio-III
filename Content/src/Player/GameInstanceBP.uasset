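; Game instance Blueprint that holds the player's experience, wallet and card deck state.
; Experience accumulates as one running total, from which level is derived by division and current progress by modulo against ExperienceLimit.
; Wallet additions are capped at WalletLimit.
; DrawCard returns the deck card at NextDrawIndex without advancing it, while IncreaseIndex separately steps that index and wraps it to the start.
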(fn UpdateExperience
  (params (ExperienceToBeAdded :type Integer))
  (Variables|Default|SetExperience (+ (Variables|Default|GetExperience) ExperienceToBeAdded)))

(fn GetLevel
  (bind _result (Math|Integer|IncrementInt (/ (Variables|Default|GetExperience) (Variables|Default|GetExperienceLimit)))
    (:%20%20
      (return _result))))

(fn UpdateWallet
  (params (AmountToBeAdded :type Integer))
  (bind _walletlimit (Variables|Default|GetWalletLimit))
  (if (>= (+ (Variables|Default|GetWallet) AmountToBeAdded) _walletlimit)
    (Variables|Default|SetWallet _walletlimit)
    (else
      (Variables|Default|SetWallet (+ (Variables|Default|GetWallet) AmountToBeAdded)))))

(fn GetExperience
  (return (Math|Integer|%(Integer) (Variables|Default|GetExperience) (Variables|Default|GetExperienceLimit))))

(fn IncreaseIndex
  (bind _result (Math|Integer|IncrementInt (Variables|Default|GetNextDrawIndex))
    (:%20%20
      (if (> _result (Utilities|Array|LastIndex (Variables|Default|GetList%20OfCardsInDeck)))
        (Variables|Default|SetNextDrawIndex 0)
        (else
          (Variables|Default|SetNextDrawIndex _result))))))

(fn DrawCard
  (return (Utilities|Array|Get(acopy) (Variables|Default|GetList%20OfCardsInDeck) (Variables|Default|GetNextDrawIndex))))